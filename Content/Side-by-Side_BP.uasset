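; Side-by-side stereo 3D controller that toggles stereo rendering and tunes eye offset, projection plane offset and FOV through input actions.
; Tick applies held-key offset changes along a logarithmic ramp, with Left Shift flipping direction; other keys reset or flip between preset values.
; FOV steps also apply to CharacterCamera when valid.
; Stereo switches update screen resolution through a macro that halves the vertical resolution while stereo is on.
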(event `self.ReceiveBeginPlay`
  (`|ExecutionSequence`
    (:`then_0`
      (`SideBySideBPLibrary.SetIsEditor` (`self.bIsInEditor`)))
    (:`then_1`
      (`SideBySideBPLibrary.EnableStereo` (`self.bIsStereoEnabled`)))
    (:`then_2`
      ;[1 1 1] adjust res if stereo is on
      (bind _returnvalue (`SideBySideBPLibrary.IsStereoEnabled`))
      (if _returnvalue
        (`self.M_AdjustResolution` _returnvalue)))))

(event `self.ReceiveTick`
  (params (DeltaSeconds :type "Float (single-precision)"))
  ;[1 1 1] Tick
  (`|ExecutionSequence`
    (:`then_0`
      (`self.UpdateEyeOffset`))
    (:`then_1`
      (`self.UpdateProjPlaneOffset`))))

(event `InputAction|EyeOffset`
  (params (Key :type "Key Structure"))
  ;[1 1 1] +/- eye offset
  (:`Pressed`
    (set `self.bIsEyeKeyPressed` true)
    (set `self.OffsetValue` (`self.StartOffsetEye`)))
  (:`Released`
    (set `self.bIsEyeKeyPressed` false)
    (set `self.OffsetValue` (`self.DefaultOffsetValue`))))

(event `Key|LeftShift`
  (params (Key :type "Key Structure"))
  ;[1 1 1] Invert Offset
  (:`Pressed`
    (set `self.bIsOffsetModifierPressed` true))
  (:`Released`
    (set `self.bIsOffsetModifierPressed` false)))

(event `InputAction|ProjectionOffset`
  (params (Key :type "Key Structure"))
  ;[1 1 1] +/- projection offset
  (:`Pressed`
    (set `self.bIsProjKeyPressed` true))
  (:`Released`
    (set `self.bIsProjKeyPressed` false)
    (set `self.OffsetValue` (`self.DefaultOffsetValue`))))

(event `InputAction|Reset`
  (params (Key :type "Key Structure"))
  ;[1 1 1] Reset
  (:`Pressed`
    (`SideBySideBPLibrary.SetProjectionPlaneOffset` 0.151976421)
    (`SideBySideBPLibrary.SetEyeOffset` "3.2000005f")))

(event `InputAction|Show Debug Messages`
  (params (Key :type "Key Structure"))
  ;[1 1 1] show debug messages
  (:`Pressed`
    (bind _isa (`/Engine/EditorBlueprintResources/StandardMacros.FlipFlop`)
      (:`A`
        _)
      (:`B`
        _))
    (`SideBySideBPLibrary.SetShowDebugMessage` _isa)))

(event `InputAction|Default 1`
  (params (Key :type "Key Structure"))
  ;[1 1 1] Defaults
  (:`Pressed`
    (`/Engine/EditorBlueprintResources/StandardMacros.FlipFlop`
      (:`A`
        (`SideBySideBPLibrary.SetProjectionPlaneOffset` 0.03))
      (:`B`
        (`SideBySideBPLibrary.SetProjectionPlaneOffset` 0.151976421)))))

(event `InputAction|Default 2`
  (params (Key :type "Key Structure"))
  ;[1 1 1] Defaults
  (:`Pressed`
    (`/Engine/EditorBlueprintResources/StandardMacros.FlipFlop`
      (:`A`
        (`SideBySideBPLibrary.SetEyeOffset` 0.0))
      (:`B`
        (`SideBySideBPLibrary.SetEyeOffset` " 3.20000005f")))))

(event `InputAction|DecFOV`
  (params (Key :type "Key Structure"))
  (bind _charactercamera (`self.CharacterCamera`))
  ;[1 1 1] +/- FOV
  (:`Pressed`
    (`SideBySideBPLibrary.DecFOV` (`self.FOVOffset`))
    (`/Engine/EditorBlueprintResources/StandardMacros.IsValid` _charactercamera
      (:`Is Valid`
        (`CameraComponent.SetFieldOfView` _charactercamera (- (`CameraComponent.FieldOfView` _charactercamera) (`self.FOVOffset`)))
        (bind _returnvalue (`SideBySideBPLibrary.GetFOV` :!label _label))
        (`KismetSystemLibrary.PrintString` (`KismetStringLibrary.Concat_StrStr` "P3D: " (`KismetStringLibrary.Conv_DoubleToString` _returnvalue)) (`self.LogToScreen`))
        (`KismetSystemLibrary.PrintString` (`KismetStringLibrary.Concat_StrStr` "S3D: " (`KismetStringLibrary.Conv_DoubleToString` (`CameraComponent.FieldOfView` (`self.CharacterCamera`)))) (`self.LogToScreen`))))))

(event `InputAction|IncFOV`
  (params (Key :type "Key Structure"))
  (bind _charactercamera (`self.CharacterCamera`))
  ;[1 1 1] +/- FOV
  (:`Pressed`
    (`SideBySideBPLibrary.IncFOV` (`self.FOVOffset`))
    (`/Engine/EditorBlueprintResources/StandardMacros.IsValid` _charactercamera
      (:`Is Valid`
        (`CameraComponent.SetFieldOfView` _charactercamera (+ (`CameraComponent.FieldOfView` _charactercamera) (`self.FOVOffset`)))
        (goto _label)))))

(event `InputAction|Toggle Stereo`
  (params (Key :type "Key Structure"))
  ;[1 1 1] Toggle Stereo
  (:`Pressed`
    (bind _isa (`/Engine/EditorBlueprintResources/StandardMacros.FlipFlop`)
      (:`A`
        _)
      (:`B`
        _))
    (`SideBySideBPLibrary.EnableStereo` _isa)
    (bind _output_get (set `self.bIsStereoEnabled` _isa))
    (`self.M_AdjustResolution` _output_get)))

(event `SetNewFOV`
  (params (`New FOV` :type "Float (double-precision)"))
  ;[1 1 1] Set FOV
  (`SideBySideBPLibrary.SetNewFOV` `New FOV`)
  (bind _returnvalue (`SideBySideBPLibrary.GetFOV`))
  (`KismetSystemLibrary.PrintString` (`KismetStringLibrary.Conv_DoubleToString` _returnvalue) (`self.LogToScreen`)))

(fn `IncrementDelta`
  (set `self.OffsetValue` (+ (`self.OffsetValue`) (`self.DefaultOffsetValue`))))

(fn `SetStereoCamera`
  (bind _outactors (`GameplayStatics.GetAllActorsOfClass` "/Script/Engine.CameraActor"))
  (for _array_element _outactors
    (bind _cameracomponent (`CameraActor.CameraComponent` _array_element))
    (bind _returnvalue (`ActorComponent.IsActive` _cameracomponent))
    (`KismetSystemLibrary.PrintString` (`KismetStringLibrary.Concat_StrStr` (`KismetSystemLibrary.GetDisplayName` _cameracomponent) (`KismetStringLibrary.Conv_BoolToString` _returnvalue)))
    (if _returnvalue
      (set `self.CharacterCamera` _cameracomponent)
      (break))))

(fn `UpdateEyeOffset`
  (bind _returnvalue (`KismetMathLibrary.Loge` (+ (`self.OffsetValue`) 1.0)))
  (bind _returnvalue_2 (* (`KismetMathLibrary.Loge` (+ (`self.OffsetValue`) 1.0)) -1.0))
  (if (`self.bIsEyeKeyPressed`)
    (if (`self.bIsOffsetModifierPressed`)
      (`SideBySideBPLibrary.SetEyeOffsetWithDelta` _returnvalue)
      (`KismetSystemLibrary.PrintString` (`KismetStringLibrary.Conv_DoubleToString` _returnvalue) true true (struct :`G` 0.051178 :`B` 1.0 :`A` 1.0) 0.0)
      (else
        (`SideBySideBPLibrary.SetEyeOffsetWithDelta` _returnvalue_2)
        (`KismetSystemLibrary.PrintString` (`KismetStringLibrary.Conv_DoubleToString` _returnvalue_2) true true (struct :`R` 1.0 :`B` 0.954412 :`A` 1.0) 0.0)))
    (`self.IncrementDelta`)))

(fn `UpdateProjPlaneOffset`
  (bind _returnvalue (`KismetMathLibrary.Loge` (+ (`self.OffsetValue`) 1.0)))
  (bind _returnvalue_2 (* _returnvalue -1.0))
  (if (`self.bIsProjKeyPressed`)
    (if (`self.bIsOffsetModifierPressed`)
      (`SideBySideBPLibrary.SetProjectionPlaneOffsetWithDelta` _returnvalue)
      (`KismetSystemLibrary.PrintString` (`KismetStringLibrary.Conv_DoubleToString` _returnvalue) true true (struct :`R` 0.099998 :`G` 0.205036 :`B` 1.0 :`A` 1.0) 0.0)
      (else
        (`SideBySideBPLibrary.SetProjectionPlaneOffsetWithDelta` _returnvalue_2)
        (`KismetSystemLibrary.PrintString` (`KismetStringLibrary.Conv_DoubleToString` _returnvalue_2) true true (struct :`R` 1.0 :`G` 0.241298 :`B` 0.351137 :`A` 1.0) 0.0)))
    (`self.IncrementDelta`)))

(fn `UserConstructionScript`)